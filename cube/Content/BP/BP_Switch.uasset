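; BP_Switch is a hit-activated switch that toggles the gates in its tag group.
; On BeginPlay it caches every actor carrying its TagName.
; Each hit on Gate_Switch flips its Status, swaps its material between red and blue, and inverts GateStatus on each cached BP_Gate, with no filter on what hit it.
; A branch touching Status for cached BP_Switch actors is disconnected and never runs.
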(event OnComponentHit(Gate_Switch)
  (params (HitComponent :type Primitive%20Component%20Object%20Reference) (OtherActor :type Actor%20Object%20Reference) (OtherComp :type Primitive%20Component%20Object%20Reference) (NormalImpulse :type Vector :default "0, 0, 0") (Hit :type Hit%20Result%20Structure%20%28by%20ref%29))
  (bind _as_bp_gate (Variables|Default|GetAs%20BP%20Gate))
  (if (Variables|Default|Getstatus)
    (Variables|Default|Setstatus false)
    (Rendering|Material|SetMaterial (Variables|Default|GetGate_Switch) 1 "/Game/Material/Gate/M_Switch_Blue.M_Switch_Blue")
    (else
      (Variables|Default|Setstatus true)
      (Rendering|Material|SetMaterial (Variables|Default|GetGate_Switch) 1 "/Game/Material/Gate/M_Switch_Red.M_Switch_Red")))
  (if (Utilities|Array|IsValidIndex (Variables|Default|GetSameGroupGates))
    (for _array_element (Variables|Default|GetSameGroupGates)
      (bind _output_get (Variables|Default|SetArray%20Element _array_element))
      (if (== (Utilities|GetClass _output_get) "/Game/BP/BP_Gate.BP_Gate_C")
        (bind _asbp_gate (Utilities|Casting|CastToBP_Gate (Variables|Default|GetArray%20Element)))
        (if (Variables|/Game/BP/BP_Gate.BP_Gate_C|GetGateStatus _asbp_gate)
          (Variables|/Game/BP/BP_Gate.BP_Gate_C|SetGateStatus _as_bp_gate false)
          (else
            (Variables|/Game/BP/BP_Gate.BP_Gate_C|SetGateStatus _as_bp_gate true)))))))

(event EventBeginPlay
  ;[1 1 1] 同じ色のゲートの情報を取得
  (bind _outactors (Actor|GetAllActorswithTag (Variables|Default|GetTagName)))
  (Variables|Default|SetSameGroupGates _outactors))

(fn ConstructionScript)