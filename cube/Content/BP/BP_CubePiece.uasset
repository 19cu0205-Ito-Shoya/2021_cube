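; BP_CubePiece is a selectable cube block that shows hover and selection states by swapping outline materials.
; Hover highlights and selection apply only while the player controller's CanMove and CanCubeCameraMove are both off.
; Clicking reports the piece to the controlled BP_StageCube pawn and toggles SelectNow and DeselectGuide.
; ChooseOtherBlock clears the selection, while ModeChanged resets only the material.
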(event OnClicked(Cube)
  (params (TouchedComponent :type Primitive%20Component%20Object%20Reference) (ButtonPressed :type Key%20Structure :default "None"))
  (bind _returnvalue (Game|GetPlayerController 0))
  ;[1 1 1] ブロック選択時
  (if (Variables|Default|GetselectNow)
    (Rendering|Material|SetMaterial (Variables|Default|GetCube) 0 "/Game/Material/OutLine_V.OutLine_V")
    (Variables|Default|SetselectNow false)
    (Variables|Default|SetDeselectGuide true)
    (bind _asbp_stage_cube (Utilities|Casting|CastToBP_StageCube (Pawn|GetControlledPawn (Game|GetPlayerController 0))))
    (Variables|/Game/BP/BP_StageCube.BP_StageCube_C|SetSelectedCube _asbp_stage_cube false)
    (else
      (Variables|Default|SetCube_Position (Transformation|GetActorTransform))
      (bind _asbp_stage_cube_2 (Utilities|Casting|CastToBP_StageCube (Pawn|GetControlledPawn _returnvalue)))
      (Default|ChoosedBlock _asbp_stage_cube_2 self)
      (bind _asplayercontroller (Utilities|Casting|CastToplayercontroller _returnvalue))
      (if (not (Variables|/Game/playercontroller.playercontroller_C|GetCanMove _asplayercontroller))
        (if (not (Variables|/Game/playercontroller.playercontroller_C|GetCanCubeCameraMove _asplayercontroller))
          (Rendering|Material|SetMaterial (Variables|Default|GetCube) 0 "/Game/Material/OutLine_select.OutLine_select")
          (Variables|Default|SetselectNow true)
          (Variables|Default|SetDeselectGuide false)
          (Development|PrintString "selectnow::"))))))

(event OnBeginCursorOver(Cube)
  (params (TouchedComponent :type Primitive%20Component%20Object%20Reference))
  ;[1 1 1] カーソル合わせた時にわかりやすくする
  (bind _asplayercontroller (Utilities|Casting|CastToplayercontroller (Game|GetPlayerController 0)))
  (if (not (Variables|/Game/playercontroller.playercontroller_C|GetCanMove _asplayercontroller))
    (if (not (Variables|/Game/playercontroller.playercontroller_C|GetCanCubeCameraMove _asplayercontroller))
      (Rendering|Material|SetMaterial (Variables|Default|GetCube) 0 "/Game/Material/OutLine_V2.OutLine_V2"))))

(event OnEndCursorOver(Cube)
  (params (TouchedComponent :type Primitive%20Component%20Object%20Reference))
  (bind _cube (Variables|Default|GetCube))
  ;[1 1 1] カーソル合わせた時にわかりやすくする
  (bind _asplayercontroller (Utilities|Casting|CastToplayercontroller (Game|GetPlayerController 0)))
  (if (not (Variables|/Game/playercontroller.playercontroller_C|GetCanMove _asplayercontroller))
    (if (not (Variables|/Game/playercontroller.playercontroller_C|GetCanCubeCameraMove _asplayercontroller))
      (if (Variables|Default|GetselectNow)
        (Rendering|Material|SetMaterial _cube 0 "/Game/Material/OutLine_select.OutLine_select")
        (else
          (Rendering|Material|SetMaterial _cube 0 "/Game/Material/OutLine_V.OutLine_V"))))))

(event Custom|ChooseOtherBlock
  (params (BlockName :type String))
  ;[1 1 1] 他のブロックを選択時
  (Rendering|Material|SetMaterial (Variables|Default|GetCube) 0 "/Game/a/OutLine_V.OutLine_V")
  (Variables|Default|SetselectNow false)
  (Variables|Default|SetDeselectGuide true))

(fn ConstructionScript)

(fn ModeChanged
  (Rendering|Material|SetMaterial (Variables|Default|GetCube) 0 "/Game/Material/OutLine_V.OutLine_V"))