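; BP_CursorEffect spawns a tiny Trail_NS Niagara effect where the moving mouse cursor passes over Pawn-type objects in the world.
; On Tick it acts only if the mouse has moved, the left button is not held and the camera's summed absolute coordinates reach a distance threshold from the origin.
; It deprojects the cursor, line-traces for Pawn objects and spawns the system at the impact point.
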(event EventTick
  (params (DeltaSeconds :type Float%20%28single-precision%29))
  (bind _returnvalue (Game|GetPlayerController 0))
  (bind (_locationx _locationy) (Game|Player|GetMousePosition _returnvalue))
  (bind (_locationx_2 _locationy_2) (Game|Player|GetMousePosition _returnvalue))
  (bind _playercameramanager (Variables|/Script/Engine.PlayerController|GetPlayerCameraManager _returnvalue))
  (bind (_worldlocation _worlddirection) (Class|PlayerController|DeprojectScreenPositiontoWorld _returnvalue _locationx _locationy))
  (bind _returnvalue_2 (Camera|GetCameraLocation _playercameramanager))
  (Variables|Default|SetMousePos (Math|Vector|MakeVector _locationx_2 _locationy_2 0.0))
  (if (not (Math|Vector|Equal(Vector) (Variables|Default|GetMousePos) (Variables|Default|GetMousePos2) 0.0001))
    (Variables|Default|SetMousePos2 (Variables|Default|GetMousePos))
    (if (>= (+ (Math|Float|Absolute(Float) (.x _returnvalue_2)) (Math|Float|Absolute(Float) (.y _returnvalue_2)) (Math|Float|Absolute(Float) (.z _returnvalue_2))) 5e+02)
      (if (not (== (Class|PlayerController|GetInputAnalogKeyState (Game|GetPlayerController 0) "LeftMouseButton") 1.0))
        (bind (_outhit _returnvalue_3) (Collision|LineTraceForObjects _worldlocation (+ _worldlocation (* _worlddirection 1e+04)) (Utilities|Array|MakeArray "ObjectTypeQuery3") false 0 "None" true "(R=1.000000,G=0.000000,B=0.000000,A=1.000000)" "(R=0.000000,G=1.000000,B=0.000000,A=1.000000)" 2.0))
        (if _returnvalue_3
          (Niagara|SpawnSystematLocation "/Game/Effect/Trail/Trail_NS.Trail_NS" (.ImpactPoint (Collision|BreakHitResult _outhit)) "0, 0, 0" "0.010000,0.010000,0.010000"))))))

(fn ConstructionScript)