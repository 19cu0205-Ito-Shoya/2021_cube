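; BP_chara1 is a player character with camera-yaw-relative movement gated by CanMove, a beehive counter and a dialogue text box.
; Losing a beehive decrements the count and spawns BP_Beehive at the character.
; Dialogue creates a TextBox widget (C key for testing), advancing through data-table rows behind a delay-reset DoOnce until the conversation flag ends.
; Box overlaps tell BP_CubeUnit whether the player is on it.
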(event OnComponentBeginOverlap(Box)
  (params (OverlappedComponent :type Primitive%20Component%20Object%20Reference) (OtherActor :type Actor%20Object%20Reference) (OtherComp :type Primitive%20Component%20Object%20Reference) (OtherBodyIndex :type Integer) (bFromSweep :type Boolean) (SweepResult :type Hit%20Result%20Structure%20%28by%20ref%29))
  (if (== (Utilities|GetClass OtherActor) "/Game/BP/BP_CubeUnit.BP_CubeUnit_C")
    (bind _asbp_cube_unit (Utilities|Casting|CastToBP_CubeUnit OtherActor))
    (Class|CubeUnit|SetPlayerIsonCubeUnit _asbp_cube_unit true)))

(event OnComponentEndOverlap(Box)
  (params (OverlappedComponent :type Primitive%20Component%20Object%20Reference) (OtherActor :type Actor%20Object%20Reference) (OtherComp :type Primitive%20Component%20Object%20Reference) (OtherBodyIndex :type Integer))
  (if (== (Utilities|GetClass OtherActor) "/Game/BP/BP_CubeUnit.BP_CubeUnit_C")
    (bind _asbp_cube_unit (Utilities|Casting|CastToBP_CubeUnit OtherActor))
    (Class|CubeUnit|SetPlayerIsonCubeUnit _asbp_cube_unit false)))

(event Custom|CallTextWidget
  (params (DialogueTableName :type Data%20Table%20Object%20Reference))
  ;[1 1 1] 文字送りの機能
  ;;[1 1 1] TEXTWidgetの生成
  (Utilities|IsValid (Variables|Default|GetTextBox)
    (:Is%20Not%20Valid
      (Variables|Default|SetDialogue%20Table%20Name DialogueTableName)
      (bind _returnvalue (UserInterface|CreateWidget "/Game/Dialogue/TextBox.TextBox_C"))
      (bind _output_get (Variables|Default|SetTextBox _returnvalue))
      (UserInterface|Viewport|AddtoViewport _output_get 0)
      (Utilities|FlowControl|Delay 0.5)
      (bind _dialogue (CallFunction|LordDialogueData (Variables|Default|GetNum) (Variables|Default|GetDialogue%20Table%20Name)))
      (Default|SetupStringChar (Variables|Default|GetTextBox) _dialogue)
      (Utilities|FlowControl|Delay 4.0)
      (Utilities|FlowControl|DoOnce true) ; enters at Reset
    )))

(event Custom|ContinueDialogue
  ;[1 1 1] 文字送りの機能
  (Utilities|IsValid (Variables|Default|GetTextBox)
    (:Is%20Valid
      (Utilities|FlowControl|DoOnce true :!label _label
        (:Completed
          (for _array_element (Variables|/Game/Dialogue/TextBox.TextBox_C|GetHoriArray (Variables|Default|GetTextBox))
            (Widget|Panel|ClearChildren _array_element))
          (bind _output_get (Variables|Default|SetNum (+ (Variables|Default|GetNum) 1)))
          (bind (_conversation _dialogue) (CallFunction|LordDialogueData _output_get (Variables|Default|GetDialogue%20Table%20Name)))
          (if _conversation
            (Default|SetupStringChar (Variables|Default|GetTextBox) _dialogue)
            (Utilities|FlowControl|Delay 4.0)
            (goto _label Reset)
            (else
              (Widget|RemovefromParent (Variables|Default|GetTextBox)))))))))

(event Custom|GetBeehive
  ;[1 1 1] Beehive collide event by shu
  (Math|Integer|IncrementInt (Variables|Default|GetBeehiveNumber)
    (:%20%20
      (Development|PrintString "Beehive Num inc"))))

(event Custom|LostBeehive
  ;[1 1 1] Beehive collide event by shu
  (if (> (Variables|Default|GetBeehiveNumber) 0)
    (Math|Integer|DecrementInt (Variables|Default|GetBeehiveNumber)
      (:%20%20
        (Game|SpawnActorfromClass "/Game/BP/BP_Beehive.BP_Beehive_C" (Transformation|GetActorTransform self) "Undefined" 0 0)))))

(event Input|AxisEvents|InputAxisMoveForward
  (params (AxisValue :type Float%20%28single-precision%29))
  ;[1 1 1] 移動
  (if (Variables|Default|GetCanMove)
    (Pawn|Input|AddMovementInput (Math|Vector|GetForwardVector (Math|Rotator|MakeRotator 0.0 0.0 (.Yaw (Math|Rotator|BreakRotator (Pawn|GetControlRotation :!class /Script/Engine.Pawn))))) AxisValue false)))

(event Input|AxisEvents|InputAxisMoveRight
  (params (AxisValue :type Float%20%28single-precision%29))
  ;[1 1 1] 移動
  (if (Variables|Default|GetCanMove)
    (Pawn|Input|AddMovementInput (Math|Vector|GetRightVector (Math|Rotator|MakeRotator 0.0 0.0 (.Yaw (Math|Rotator|BreakRotator (Pawn|GetControlRotation :!class /Script/Engine.Pawn))))) AxisValue false)))

(event Input|KeyboardEvents|Right
  (params (Key :type Key%20Structure :default "None")))

(event Input|KeyboardEvents|Left
  (params (Key :type Key%20Structure :default "None")))

(event Input|MouseEvents|RightMouseButton
  (params (Key :type Key%20Structure :default "None")))

(event Input|MouseEvents|LeftMouseButton
  (params (Key :type Key%20Structure :default "None")))

(event Input|KeyboardEvents|C
  (params (Key :type Key%20Structure :default "None"))
  ;[1 1 1] テスト用(文字送りの機能呼び出し)
  (:Pressed
    (CallFunction|CallTextWidget "/Game/Dialogue/Dialogue.Dialogue")))

(fn ConstructionScript)