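; Gate actor built from four BP_GateCube child actors, with vertical movement and state driven by GateStatus.
; Each Tick it steps two of the cubes along Z, using the start heights of all four, recorded at BeginPlay, as thresholds.
; Cross-resetting DoOnce nodes toggle actor collision as movement checks fail and set every child cube's Status when GateStatus changes.
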(event EventBeginPlay
  (Variables|Default|SetDefaultLoc (Transformation|GetWorldLocation (Variables|Default|GetBP_GateCube)))
  (Variables|Default|SetDefaultLoc_1 (Transformation|GetWorldLocation (Variables|Default|GetBP_GateCube1)))
  (Variables|Default|SetDefaultLoc_2 (Transformation|GetWorldLocation (Variables|Default|GetBP_GateCube2)))
  (Variables|Default|SetDefaultLoc_3 (Transformation|GetWorldLocation (Variables|Default|GetBP_GateCube3)))
  (Variables|Default|SetArray (Utilities|Array|MakeArray (Variables|Default|GetBP_GateCube) (Variables|Default|GetBP_GateCube1) (Variables|Default|GetBP_GateCube2) (Variables|Default|GetBP_GateCube3))))

(event EventTick
  (params (DeltaSeconds :type Float%20%28single-precision%29))
  (bind _bp_gatecube (Variables|Default|GetBP_GateCube))
  (bind _bp_gatecube1 (Variables|Default|GetBP_GateCube1))
  (bind _bp_gatecube_2 (Variables|Default|GetBP_GateCube))
  (bind _bp_gatecube1_2 (Variables|Default|GetBP_GateCube1))
  (if (Variables|Default|GetGateStatus)
    (Utilities|FlowControl|Sequence
      (:then_0
        (if (|CollapseGraph_0)
          (Transformation|SetWorldLocation _bp_gatecube (+ (Transformation|GetWorldLocation _bp_gatecube) "0, 0,1.000000") false false))
        (if (|CollapseGraph_1)
          (Transformation|SetWorldLocation _bp_gatecube1 (+ (Transformation|GetWorldLocation _bp_gatecube1) "0, 0,1.000000") false false)
          (else
            (Utilities|FlowControl|DoOnce false :!label _label
              (:Completed
                (Collision|SetActorEnableCollision true)
                (goto _label_4 Reset))))))
      (:then_1
        (Utilities|FlowControl|DoOnce false :!label _label_2
          (:Completed
            (for _array_element (Variables|Default|GetArray)
              (bind _asbp_gate_cube (Utilities|Casting|CastToBP_GateCube (Variables|/Script/Engine.ChildActorComponent|GetChildActor _array_element)))
              (Variables|/Game/BP/BP_GateCube.BP_GateCube_C|Setstatus _asbp_gate_cube true)
              (goto _label_3 Reset))))))
    (else
      (Utilities|FlowControl|Sequence
        (:then_0
          (Utilities|FlowControl|DoOnce false :!label _label_3
            (:Completed
              (for _array_element_2 (Variables|Default|GetArray)
                (bind _asbp_gate_cube_2 (Utilities|Casting|CastToBP_GateCube (Variables|/Script/Engine.ChildActorComponent|GetChildActor _array_element_2)))
                (Variables|/Game/BP/BP_GateCube.BP_GateCube_C|Setstatus _asbp_gate_cube_2 false)
                (goto _label_2 Reset)))))
        (:then_1
          (if (> (.z (Transformation|GetWorldLocation (Variables|Default|GetBP_GateCube))) (.z (Variables|Default|GetDefaultLoc_2)))
            (Transformation|SetWorldLocation _bp_gatecube_2 (+ (Transformation|GetWorldLocation _bp_gatecube_2) "0, 0,1.000000") false false))
          (if (> (.z (Transformation|GetWorldLocation (Variables|Default|GetBP_GateCube1))) (.z (Variables|Default|GetDefaultLoc_3)))
            (Transformation|SetWorldLocation _bp_gatecube1_2 (+ (Transformation|GetWorldLocation _bp_gatecube1_2) "0, 0,1.000000") false false)
            (else
              (Utilities|FlowControl|DoOnce false :!label _label_4
                (:Completed
                  (Collision|SetActorEnableCollision false)
                  (goto _label Reset))))))))))

(fn ConstructionScript)