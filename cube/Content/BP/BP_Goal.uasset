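; BP_Goal is the stage goal actor that ends a stage when the player character reaches it.
; On overlap with a BP_chara, a DoOnce gate sets the character's IsStageClear flag and shows the Clear widget.
; A timed sequence then calls FadeOut and, after a further delay, loads the StageSelect level.
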(event EventBeginPlay)

(event Collision|EventActorBeginOverlap
  (params (OtherActor :type Actor%20Object%20Reference))
  (bind _asbp_chara (Utilities|Casting|CastToBP_chara OtherActor))
  (Utilities|FlowControl|DoOnce false
    (:Completed
      (Variables|/Game/BP/BP_chara.BP_chara_C|SetIsStageClear _asbp_chara true)
      (Utilities|FlowControl|Sequence
        (:then_0
          (bind _returnvalue (UserInterface|CreateWidget "/Game/Widget/Clear/Clear.Clear_C"))
          (bind _output_get (Variables|Default|SetGameClear _returnvalue))
          (UserInterface|Viewport|AddtoViewport _output_get 0))
        (:then_1
          (Utilities|FlowControl|Delay 3.5)
          (CallFunction|FadeOut)
          (Utilities|FlowControl|Delay 1.5)
          (Game|OpenLevel(byName) "StageSelect"))))))

(event EventTick
  (params (DeltaSeconds :type Float%20%28single-precision%29)))

(fn ConstructionScript)