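; BP_LevitatingCube is a tumbling cube that drifts toward the world origin along X, then Y, at Speed.
; Tick adds RollPower to its rotation and offsets it until both axes are near zero.
; A box overlap passing a self-comparison check spawns the Shoot effect and moves the cube to a random distant axis point.
; RandomInteger(3) never yields 3, so the fourth point, on negative Y, is unreachable.
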(event OnComponentBeginOverlap(Box)
  (params (OverlappedComponent :type Primitive%20Component%20Object%20Reference) (OtherActor :type Actor%20Object%20Reference) (OtherComp :type Primitive%20Component%20Object%20Reference) (OtherBodyIndex :type Integer) (bFromSweep :type Boolean) (SweepResult :type Hit%20Result%20Structure%20%28by%20ref%29))
  (bind _self self)
  (bind _cube (Variables|Default|GetCube))
  (bind _returnvalue (Transformation|GetWorldLocation _cube))
  (if (or (== OverlappedComponent _self) (== OtherActor _self))
    (Niagara|SpawnSystematLocation "/Game/BP/Holl/ShootEffect/Shoot.Shoot" (Math|Vector|MakeVector (.x _returnvalue) (.y _returnvalue) (.z _returnvalue)))
    (switch int (Math|Random|RandomInteger 3)
      (:0
        (Variables|Default|SetTelePosition "2600.000000,0.000000,-200.000000"))
      (:1
        (Variables|Default|SetTelePosition "-2600.000000,0.000000,-200.000000"))
      (:2
        (Variables|Default|SetTelePosition "0.000000,2600.000000,-200.000000"))
      (:3
        (Variables|Default|SetTelePosition "0.000000,-2600.000000,-200.000000")))
    (Transformation|SetWorldLocation (Variables|Default|GetCube) (Variables|Default|GetTelePosition) false false)))

(event EventTick
  (params (DeltaSeconds :type Float%20%28single-precision%29))
  (bind _cube (Variables|Default|GetCube))
  (bind _rollpower (Variables|Default|GetRollPower))
  (bind _returnvalue (Transformation|GetWorldLocation _cube))
  (Transformation|SetRelativeRotation (Variables|Default|GetCube) (Math|Rotator|CombineRotators (Transformation|GetWorldRotation (Variables|Default|GetCube)) (Math|Rotator|MakeRotator _rollpower _rollpower _rollpower)) false false)
  (if (>= (.x _returnvalue) 1e+01)
    (Transformation|AddWorldOffset (Variables|Default|GetCube) (Math|Vector|MakeVector (* (Variables|Default|Getspeed) -1.0) 0.0 0.0) false false)
    (elif (<= (.x _returnvalue) -1e+01)
      (Transformation|AddWorldOffset (Variables|Default|GetCube) (Math|Vector|MakeVector (Variables|Default|Getspeed) 0.0 0.0) false false)
      (elif (>= (.y _returnvalue) 1e+01)
        (Transformation|AddWorldOffset (Variables|Default|GetCube) (Math|Vector|MakeVector 0.0 (* (Variables|Default|Getspeed) -1.0) 0.0) false false)
        (elif (<= (.y _returnvalue) -1e+01)
          (Transformation|AddWorldOffset (Variables|Default|GetCube) (Math|Vector|MakeVector 0.0 (Variables|Default|Getspeed) 0.0) false false))))))

(fn ConstructionScript)