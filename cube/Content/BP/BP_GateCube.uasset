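; BP_GateCube is a cube that spins while its Status flag is true.
; Each Tick adds the per-axis RollPower values to the Cube's world rotation through CombineRotators.
; Two DoOnce nodes that reset each other set the material in slot 0 once per Status change instead of every frame.
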(event EventTick
  (params (DeltaSeconds :type Float%20%28single-precision%29))
  (if (Variables|Default|Getstatus)
    (Utilities|FlowControl|Sequence
      (:then_0
        (Transformation|SetWorldRotation (Variables|Default|GetCube) (Math|Rotator|CombineRotators (Transformation|GetWorldRotation (Variables|Default|GetCube)) (Math|Rotator|MakeRotator (Variables|Default|GetRollPower_X) (Variables|Default|GetRollPower_Y) (Variables|Default|GetRollPower_Z))) false false))
      (:then_1
        (Utilities|FlowControl|DoOnce false :!label _label
          (:Completed
            (Rendering|Material|SetMaterial (Variables|Default|GetCube) 0 0)
            (goto _label_2 Reset)))))
    (else
      (Utilities|FlowControl|DoOnce false :!label _label_2
        (:Completed
          (Rendering|Material|SetMaterial (Variables|Default|GetCube) 0 0)
          (goto _label Reset))))))

(fn ConstructionScript)