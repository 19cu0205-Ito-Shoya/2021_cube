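; Character Blueprint that tracks how many beehives the character carries.
; GetBeehive increments the count, while LostBeehive decrements it when above zero and spawns a BP_Beehive at the character's transform.
; The movement axis events are empty.
; Yaw-relative movement gated by CanMove and view-target switching between self and Cube remain as disconnected, unexecuted nodes.
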(event Custom|GetBeehive
  (Math|Integer|IncrementInt (Variables|Default|GetBeehiveNumber)
    (:%20%20
      (Development|PrintString "Beehive Num inc"))))

(event Custom|LostBeehive
  (if (> (Variables|Default|GetBeehiveNumber) 0)
    (Math|Integer|DecrementInt (Variables|Default|GetBeehiveNumber)
      (:%20%20
        (Game|SpawnActorfromClass "/Game/BP/BP_Beehive.BP_Beehive_C" (Transformation|GetActorTransform self) "Undefined" 0 0)))))

(event Input|AxisEvents|InputAxisMoveForward
  (params (AxisValue :type Float%20%28single-precision%29))
  ;[1 1 1] 移動
)

(event Input|AxisEvents|InputAxisMoveRight
  (params (AxisValue :type Float%20%28single-precision%29))
  ;[1 1 1] 移動
)

(event Input|KeyboardEvents|Right
  (params (Key :type Key%20Structure :default "None")))

(event Input|KeyboardEvents|Left
  (params (Key :type Key%20Structure :default "None")))

(event Input|MouseEvents|RightMouseButton
  (params (Key :type Key%20Structure :default "None")))

(event Input|MouseEvents|LeftMouseButton
  (params (Key :type Key%20Structure :default "None")))

(fn ConstructionScript)