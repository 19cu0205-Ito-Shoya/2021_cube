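; Ghost AI Blueprint, still mostly a stub, with a capsule component and a helper for finding what it stands on.
; GetStandCube0 line-traces a short distance down from the capsule along its up vector on the Visibility channel and returns the hit actor.
; BeginPlay only prints the player character's display name, while SwitchMode, Tick and overlap events have no logic.
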(event Custom|SwitchMode
  (params (value :type Boolean)))

(event EventBeginPlay
  (Development|PrintString (Utilities|GetDisplayName (Game|GetPlayerCharacter 0))))

(event Collision|EventActorBeginOverlap
  (params (OtherActor :type Actor%20Object%20Reference)))

(event EventTick
  (params (DeltaSeconds :type Float%20%28single-precision%29)))

(fn ConstructionScript)

(fn GetStandCube0
  (bind _capsulecomponent (Variables|Default|GetCapsuleComponent))
  (bind _returnvalue (Transformation|GetWorldLocation _capsulecomponent))
  (bind _outhit (Collision|LineTraceByChannel _returnvalue (+ _returnvalue (* (Math|Vector|GetUpVector _capsulecomponent) -1e+02)) "TraceTypeQuery1" false 0 "None"))
  (return (.HitActor (Collision|BreakHitResult _outhit))))