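; BP_Beehive is a beehive pickup that the player collects by touching it.
; After BeginPlay it waits for the HitCD delay before setting IsReady, so overlaps during that window are ignored.
; Once ready, an overlapping actor tagged Player that casts to BP_chara receives a GetBeehive call, and the beehive destroys itself.
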(event EventBeginPlay
  (Utilities|FlowControl|Delay (Variables|Default|GetHitCD))
  (Variables|Default|SetisReady true))

(event EventTick
  (params (DeltaSeconds :type Float%20%28single-precision%29)))

(event Collision|EventActorBeginOverlap
  (params (OtherActor :type Actor%20Object%20Reference))
  (if (Variables|Default|GetisReady)
    (if (Actor|ActorHasTag OtherActor "Player")
      (Development|PrintString "player get beehive ")
      (bind _asbp_chara (Utilities|Casting|CastToBP_chara OtherActor))
      (Default|GetBeehive _asbp_chara)
      (Actor|DestroyActor))))

(fn ConstructionScript)