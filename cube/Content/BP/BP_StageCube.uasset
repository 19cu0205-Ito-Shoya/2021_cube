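; BP_StageCube is a cube-puzzle stage actor referencing 26 BP_CubePiece child actors and nine ChooseLine guide actors.
; Its ChoosedBlock event is empty, and all graph logic is disconnected from execution.
; The dormant logic broadcasts the chosen block to pieces and moves guides to the selected piece's position.
; Other unwired experiments attach eight pieces to a ChooseLine for group rotation, detach that line, and rotate actors, with debug prints.
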(event Custom|ChoosedBlock
  (params (ChoosedBrockName :type String)))

(event Input|KeyboardEvents|9
  (params (Key :type Key%20Structure :default "None")))

(event Input|KeyboardEvents|Q
  (params (Key :type Key%20Structure :default "None")))

(fn ConstructionScript)