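; BP_Pawn_Menu is a menu pawn that moves its physics Sphere to a target point.
; Pressing F sets IsMove, which makes Tick call MoveToTarget with TargetTemp and MoveSpeed.
; MoveToTarget sets the Sphere's linear velocity toward the target, then zeroes it and clears IsMove once within a small tolerance.
; Debug prints mark movement start, while the "move off" branch is disconnected.
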(event EventBeginPlay)

(event Collision|EventActorBeginOverlap
  (params (OtherActor :type Actor%20Object%20Reference)))

(event EventTick
  (params (DeltaSeconds :type Float%20%28single-precision%29))
  (if (Variables|Default|GetIsMove)
    (CallFunction|MovetoTarget (Variables|Default|GetTargetTemp) (Variables|Default|GetMoveSpeed))))

(event Input|KeyboardEvents|F
  (params (Key :type Key%20Structure :default "None"))
  (:Pressed
    (Development|PrintString "move on")
    (Variables|Default|SetIsMove true)))

(fn ConstructionScript)

(fn MovetoTarget
  (params (Target :type Vector) (Speed :type Float%20%28single-precision%29))
  (Physics|SetPhysicsLinearVelocity (Variables|Default|GetSphere) (* (Math|Vector|Normalize (- Target (Transformation|GetWorldLocation (Variables|Default|GetSphere)))) Speed) false "None")
  (if (Math|Vector|VectorIsNearlyZero (- (Transformation|GetWorldLocation (Variables|Default|GetSphere)) Target) 1.0)
    (Variables|Default|SetIsMove false)
    (Physics|SetPhysicsLinearVelocity (Variables|Default|GetSphere) "0, 0, 0" false "None")))