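; Firework actor that spawns an enlarged Niagara explosion at its stored particle position on BeginPlay, with a random RGB trail color.
; A custom event receives Niagara particle data, stores each position and sweeps the collision sphere to it, with teleport enabled.
; The delayed respawn loop is disconnected, so the explosion spawns only once.
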(event Custom|CustomEvent
  (params (Data :type Array%20of%20Basic%20Particle%20Data%20Structures) (NiagaraSystem :type Niagara%20System%20Object%20Reference))
  (for _array_element Data
    (bind _output_get (Variables|Default|SetparticlePosition (.Position (Utilities|Struct|BreakBasicParticleData _array_element))))
    (bind _spherecollision (Variables|Default|GetSphereCollision)
      (:then
        (Transformation|SetWorldLocation _spherecollision _output_get true true))
      (:else))))

(event EventBeginPlay
  (bind _returnvalue (Niagara|SpawnSystematLocation "/Game/Effect/FireWorks/FireWorksExplosion.FireWorksExplosion" (Variables|Default|GetparticlePosition) "0, 0, 0" "10.000000,10.000000,10.000000"))
  (bind _output_get (Variables|Default|SetExplosion _returnvalue))
  (Niagara|SetNiagaraVariable(LinearColor) _returnvalue "TrailColor" (CallFunction|RandomColor)))

(event Collision|EventActorBeginOverlap
  (params (OtherActor :type Actor%20Object%20Reference)))

(fn ConstructionScript)

(fn RandomColor
  (return (Utilities|Struct|MakeLinearColor (Math|Random|RandomFloatinRange 0.0 1.0) (Math|Random|RandomFloatinRange 0.0 1.0) (Math|Random|RandomFloatinRange 0.0 1.0) 1.0)))