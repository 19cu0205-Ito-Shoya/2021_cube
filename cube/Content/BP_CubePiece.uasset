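; BP_CubePiece is a cube piece that can be hovered and selected with the mouse, shown by swapping its outline material.
; Hover changes the material only while the player controller's CanMove and CanCubeCameraMove are both false.
; Clicking an unselected piece applies the select material, sets SelectNow and prints the component name, without checking those flags.
; Cursor exit picks the resting material from SelectNow, which no connected logic clears.
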(event OnBeginCursorOver(Cube)
  (params (TouchedComponent :type Primitive%20Component%20Object%20Reference))
  (bind _asplayercontroller (Utilities|Casting|CastToplayercontroller (Game|GetPlayerController 0)))
  (if (not (Variables|/Game/playercontroller.playercontroller_C|GetCanMove _asplayercontroller))
    (if (not (Variables|/Game/playercontroller.playercontroller_C|GetCanCubeCameraMove _asplayercontroller))
      (Rendering|Material|SetMaterial (Variables|Default|GetCube) 0 "/Game/OutLine_H.OutLine_H"))))

(event OnEndCursorOver(Cube)
  (params (TouchedComponent :type Primitive%20Component%20Object%20Reference))
  (bind _cube (Variables|Default|GetCube))
  (bind _asplayercontroller (Utilities|Casting|CastToplayercontroller (Game|GetPlayerController 0)))
  (if (not (Variables|/Game/playercontroller.playercontroller_C|GetCanMove _asplayercontroller))
    (if (not (Variables|/Game/playercontroller.playercontroller_C|GetCanCubeCameraMove _asplayercontroller))
      (if (Variables|Default|GetselectNow)
        (Rendering|Material|SetMaterial _cube 0 "/Game/OutLine_V2.OutLine_V2")
        (else
          (Rendering|Material|SetMaterial _cube 0 "/Game/OutLine_V.OutLine_V"))))))

(event OnClicked(Cube)
  (params (TouchedComponent :type Primitive%20Component%20Object%20Reference) (ButtonPressed :type Key%20Structure :default "None"))
  (if (not (Variables|Default|GetselectNow))
    (Rendering|Material|SetMaterial (Variables|Default|GetCube) 0 "/Game/OutLine_select.OutLine_select")
    (Variables|Default|SetselectNow true)
    (Development|PrintString (Utilities|GetDisplayName TouchedComponent))))

(fn ConstructionScript)