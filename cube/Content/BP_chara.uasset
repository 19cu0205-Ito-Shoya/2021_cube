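; BP_chara is a character Blueprint with an unfinished or disabled setup for movement and view switching.
; The MoveForward and MoveRight axis events are empty, and the camera-relative planar movement logic, gated by CanMove, is disconnected.
; Two further disconnected chains switch the view target between the character and Cube, setting CanMove false and true respectively, so none of this logic runs.
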(event Input|AxisEvents|InputAxisMoveForward
  (params (AxisValue :type Float%20%28single-precision%29))
  ;[1 1 1] 移動
)

(event Input|AxisEvents|InputAxisMoveRight
  (params (AxisValue :type Float%20%28single-precision%29))
  ;[1 1 1] 移動
)

(event Input|KeyboardEvents|Right
  (params (Key :type Key%20Structure :default "None")))

(event Input|KeyboardEvents|Left
  (params (Key :type Key%20Structure :default "None")))

(event Input|MouseEvents|RightMouseButton
  (params (Key :type Key%20Structure :default "None")))

(event Input|MouseEvents|LeftMouseButton
  (params (Key :type Key%20Structure :default "None")))

(fn ConstructionScript)